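; BP_Light is a light Blueprint that blinks a SpotLight a limited number of times when play begins.
; A DoN node capped by HowMany drives a loop that shows and then hides the light, waiting Pause seconds before each change.
; The wire returns to the DoN after each blink, so blinking stops with the light hidden once the count runs out.
; A ToggleVisibility call is left unconnected.
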(event EventBeginPlay
  (Utilities|FlowControl|DoN (Variables|Default|GetHow%20many) :!label _label
    (:Exit
      (Utilities|FlowControl|Delay (Variables|Default|GetPause))
      (Rendering|SetVisibility (Variables|Default|GetSpotLight) true true)
      (Utilities|FlowControl|Delay (Variables|Default|GetPause))
      (Rendering|SetVisibility (Variables|Default|GetSpotLight) false true)
      (goto _label))))

(fn ConstructionScript)